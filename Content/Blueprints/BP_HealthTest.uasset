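; BP_HealthTest is a test Blueprint that exercises a Health component's shield and damage functions.
; On BeginPlay it adds a shield, then applies non-piercing damage that is allowed to trigger death.
; It prints CurrentHealth before and after each step; the shield value itself is never printed.
; Overlap, Tick and the construction script contain no logic.
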(event `self.ReceiveBeginPlay`
  (`KismetSystemLibrary.PrintString` (`KismetStringLibrary.Conv_DoubleToString` (`HealthComponent.CurrentHealth` (`self.Health`))))
  (`HealthComponent.AddShield` (`self.Health`) 50.0)
  (`KismetSystemLibrary.PrintString` (`KismetStringLibrary.Conv_DoubleToString` (`HealthComponent.CurrentHealth` (`self.Health`))))
  (`HealthComponent.ApplyDamage` (`self.Health`) 25.0 false true)
  (`KismetSystemLibrary.PrintString` (`KismetStringLibrary.Conv_DoubleToString` (`HealthComponent.CurrentHealth` (`self.Health`)))))

(fn `UserConstructionScript`)