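; BP_TestBoss is a test boss Blueprint that serves as a debug check on its Health object.
; On BeginPlay it prints the current health, waits one second, then prints the health again along with the IsDead result.
; It contains no combat or damage logic, and its overlap, Tick and construction script are empty.
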(event `self.ReceiveBeginPlay`
  (`KismetSystemLibrary.PrintString` (`KismetStringLibrary.Conv_DoubleToString` (`HealthComponent.CurrentHealth` (`self.Health`))))
  (`KismetSystemLibrary.Delay` 1.0)
  (`KismetSystemLibrary.PrintString` (`KismetStringLibrary.Conv_DoubleToString` (`HealthComponent.CurrentHealth` (`self.Health`))))
  (`KismetSystemLibrary.PrintString` (`KismetStringLibrary.Conv_BoolToString` (`HealthComponent.IsDead` (`self.Health`)))))

(fn `UserConstructionScript`)