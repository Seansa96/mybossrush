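; BP_GearTest is a test actor that exercises basic Inventory operations.
; On BeginPlay it adds DA_TrainingSword to its Inventory and prints the display name of the item in the first slot.
; It then moves that item to another index and prints the name at the destination, so results are checked by on-screen or log output.
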(event `self.ReceiveBeginPlay`
  (`InventoryComponent.AddItem` (`self.Inventory`) "/Game/Gear/DA_TrainingSword.DA_TrainingSword")
  (`KismetSystemLibrary.PrintString` (`KismetTextLibrary.Conv_TextToString` (`GearItemDefinition.DisplayName` (`InventoryComponent.GetItemAtIndex` (`self.Inventory`) 0))))
  (`InventoryComponent.MoveItem` (`self.Inventory`) 0 5)
  (`KismetSystemLibrary.PrintString` (`KismetTextLibrary.Conv_TextToString` (`GearItemDefinition.DisplayName` (`InventoryComponent.GetItemAtIndex` (`self.Inventory`) 5)))))

(fn `UserConstructionScript`)